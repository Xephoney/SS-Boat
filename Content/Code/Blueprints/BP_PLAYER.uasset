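; Player Blueprint that provides an orbit camera on a spring arm, with rotation and zoom controls.
; While Action 2 is held, a Gate lets Tick run CameraRotation, which turns axis input into world yaw and clamped downward pitch, scaled by sensitivity but not delta time.
; Zoom In and Zoom Out presses step the arm length by an amount scaled by ZoomSpeed, with no length limits.
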(event `self.ReceiveTick`
  (params (DeltaSeconds :type "Float (single-precision)"))
  (`|ExecutionSequence`
    (:`then_0`
      (`/Engine/EditorBlueprintResources/StandardMacros.Gate` true :!label _label
        (:`Exit`
          (`self.CameraRotation` DeltaSeconds))))))

(event `InputAction|Action 2`
  (params (Key :type "Key Structure"))
  (:`Pressed`
    (goto _label :!via `Open`))
  (:`Released`
    (goto _label :!via `Close`)))

(event `InputAction|Zoom In`
  (params (Key :type "Key Structure"))
  (:`Pressed`
    (`self.Zoom` -100.0)))

(event `InputAction|Zoom Out`
  (params (Key :type "Key Structure"))
  (:`Pressed`
    (`self.Zoom` 100.0)))

(fn `CameraRotation`
  (params (deltaSeconds :type "Float (double-precision)"))
  (locals (`Vertical sensitivity` :type "Float (double-precision)" :default 3.0) (`Horizontal Sensitivity` :type "Float (double-precision)" :default 3.0))
  (bind _springarm (`self.SpringArm`))
  (bind (_returnvalue_roll _returnvalue_pitch _returnvalue_yaw) (`KismetMathLibrary.BreakRotator` (`SceneComponent.K2_GetComponentRotation` _springarm)))
  (`SceneComponent.K2_SetWorldRotation` _springarm (`KismetMathLibrary.MakeRotator` 0.0 (`KismetMathLibrary.FClamp` (+ _returnvalue_pitch (* (`local.Vertical sensitivity`) (`self.GetInputAxisKeyValue`))) -85.0 -10.0) (+ _returnvalue_yaw (* (`self.GetInputAxisKeyValue`) (`local.Horizontal Sensitivity`)))) false false))

(fn `UserConstructionScript`)

(fn `Zoom`
  (params (Direction :type "Float (double-precision)"))
  (locals (ZoomSpeed :type "Float (double-precision)" :default 1.0))
  (bind _springarm (`self.SpringArm`))
  (set `SpringArmComponent.TargetArmLength` (+ (`SpringArmComponent.TargetArmLength` _springarm) (* Direction (`local.ZoomSpeed`))) _springarm))